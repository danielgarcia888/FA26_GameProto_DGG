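; Parent pickup actor for items the player collects in the world or purchases with coins when placed in a store.
; An ItemData asset drives its mesh, rarity-colored glow particles and optional point light in the construction script, plus its interaction data at BeginPlay.
; Interaction runs a cost check for store items, then fires OnItemPickedUp, which adds the item to inventory, plays a sound and destroys the actor on success.
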(event `self.ReceiveBeginPlay`
  (add `self.OnItemPickedUp` (delegate `OnItemPickedUp_Event`))
  ; Get interaction data structure asset // Call InitData in data asset
  (bind _itemdata (`self.ItemData`)
    (:`then`
      (set `/Game/BP/Components/AC_Interaction.InteractionData` (`/Game/BP/Data/DataAssets/000_Primary/PDA_Item. InteractionData` _itemdata) (`self.AC_Interaction`))
      (`/Game/BP/Data/DataAssets/000_Primary/PDA_Item.InitData` _itemdata self)
      (`self.ItemInStore`
        (:`then`
          ; Set interaction text for display when player character interacts with this pickup in a store
          (setmembers `/Game/BP/Data/Structs/F_InteractionData` :`StructRef` (`/Game/BP/Components/AC_Interaction.InteractionData` (`self.AC_Interaction`)) :`InteractionText` (`|FormatText` "purchase {item} for {cost} coins" (`KismetTextLibrary.TextToUpper` (`self.GetItemName`)) (`self.Cost`)) :`TriggerInteractionByTouch` false))
        (:`else`
          ; Set interaction text for display when player character interacts with this pickup in the world
          (setmembers `/Game/BP/Data/Structs/F_InteractionData` :`StructRef` (`/Game/BP/Components/AC_Interaction.InteractionData` (`self.AC_Interaction`)) :`InteractionText` (`|FormatText` "collect the {item}" (`KismetTextLibrary.TextToUpper` (`self.GetItemName`)))))))
    (:`else`)))

(event `OnItemPickedUp_Event`
  ; The bound actions that occur when OnItemPickedUp event dispatcher is called
  (bind _itemdata (`self.ItemData`)
    (:`then`
      (bind _addedsuccessfully (`/Game/BP/Data/DataAssets/000_Primary/PDA_Item.AddItemToInventory` _itemdata (`self.InteractingController`) (`self.StackSize`)))
      (if _addedsuccessfully
        (`/Game/BP/Data/DataAssets/000_Primary/PDA_Item.PlayPickupSound` _itemdata self)
        (`/Game/BP/Components/AC_Interaction.SetShowAsInteractable` (`self.AC_Interaction`) false (`self.InteractingController`))
        (`self.K2_DestroyActor`)))
    (:`else`)))

(event `self.AC_Interaction.OnInteractedWith`
  (params (InteractingController :type "PlayerController Object Reference"))
  ; Interact with pickup
  (set `self.InteractingController` InteractingController)
  (`self.ItemInStore`
    (:`then`
      ;;[0 0 0] Try to purchase the pickup item if it's in a store
      (`/Game/BP/FunctionsAndMacros/BML_Helpers.CostCheck` (`self.InteractingController`) (`self.Cost`) true
        (:`Success`
          (`self.OnItemPickedUp`))))
    (:`else`
      (`self.OnItemPickedUp`))))

(fn `GetItemName`
  (returns (Name :type Text))
  (bind _itemdata (`self.ItemData`)
    (:`then`
      (return (`.Name_2_1346FB0E4E0D52F483ACEC934DB39AE6` (break `/Game/BP/Data/Structs/F_InteractionData` (`/Game/BP/Data/DataAssets/000_Primary/PDA_Item. InteractionData` _itemdata)))))
    (:`else`)))

(fn `SetupLight`
  (bind _pointlightcomponent (`self.PointLightComponent`))
  (bind _itemdata (`self.ItemData`))
  (bind _itemdata_2 (`self.ItemData`)
    (:`then`
      (if (`/Game/BP/Data/DataAssets/000_Primary/PDA_Item.LightActive` _itemdata_2)
        (`|ExecutionSequence`
          (:`then_0`
            ; Create point light component if it's not already valid
            (`self.PointLightComponent`
              (:`then`)
              (:`else`
                (bind _returnvalue (`|AddComponentByClass` "/Script/Engine.PointLightComponent" false (`KismetMathLibrary.MakeTransform` (`KismetMathLibrary.MakeVector` 0.0 0.0 (* (`SphereComponent.SphereRadius` (`self.Collision`)) -0.9)))))
                (set `self.PointLightComponent` _returnvalue))))
          (:`then_1`
            ; Set point light attributes
            (`LocalLightComponent.SetAttenuationRadius` _pointlightcomponent 100.0)
            (`LightComponentBase.SetCastShadows` _pointlightcomponent false)
            (`LocalLightComponent.SetIntensityUnits` _pointlightcomponent "Lumens")
            (`LightComponent.SetIntensity` _pointlightcomponent (`/Game/BP/Data/DataAssets/000_Primary/PDA_Item.LightIntensity` _itemdata))
            (`LightComponent.SetLightColor` _pointlightcomponent (`/Game/BP/Data/DataAssets/000_Primary/PDA_Item.LightColor` _itemdata) true)))
        (else
          ; Destroy point light
          (bind _pointlightcomponent_2 (`self.PointLightComponent` :!label _label)
            (:`then`
              (`ActorComponent.K2_DestroyComponent` _pointlightcomponent_2))
            (:`else`)))))
    (:`else`
      (goto _label))))

(fn `SetupParticles`
  (bind _ns_pickupglow (`self.NS_PickupGlow`))
  (bind _itemdata (`self.ItemData`)
    (:`then`
      (bind ((`Rarity_30_F1070BF740E8FCD6F3638EB41805775A` _rarity)) (break `/Game/BP/Data/Structs/F_InteractionData` (`/Game/BP/Data/DataAssets/000_Primary/PDA_Item. InteractionData` _itemdata)))
      (`SceneComponent.SetHiddenInGame` _ns_pickupglow (`|EnumEquality` _rarity "NewEnumerator0") false)
      (`FXSystemComponent.SetColorParameter` _ns_pickupglow "ParticleColor" (`/Game/BP/FunctionsAndMacros/BFL_Helpers.GetColorFromRarity` _rarity)))
    (:`else`)))

(fn `UserConstructionScript`
  (`self.SetupParticles`)
  (`self.SetupLight`)
  (`/Game/BP/Data/DataAssets/000_Primary/PDA_Item.SetUpStaticMesh` (`self.ItemData`) (`self.StaticMesh`)))