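; Actor component that makes its owner interactable by look-at, overlap or touch, with highlighting and HUD prompts.
; At startup, look-at configures trace collision and an optional billboard indicator, overlap spawns a sphere notifying the player controller, and optional touch fires OnInteractedWith.
; SetShowAsInteractable toggles the highlight and keybind prompt, using a DoOnce against repeats.
; Components tagged "Interact" receive the trace block and custom-depth stencil highlight.
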(event `self.ReceiveBeginPlay`
  (`KismetSystemLibrary.DelayUntilNextTick`)
  (`|ExecutionSequence`
    (:`then_0`
      ; Settings based on interaction type
      (switch `/Game/BP/Data/Enums/E_InteractionType` (`.InteractionType_11_A22204664925E98CD6C72B9FBE34FBF6` (break `/Game/BP/Data/Structs/F_InteractionData` (`self.InteractionData`)))
        (:`NewEnumerator0`
          (setmembers `/Game/BP/Data/Structs/F_InteractionData` :`StructRef` (`self.InteractionData`) :`TriggerInteractionByTouch` false))
        (:`NewEnumerator1`
          ;;[0 0 0] Setup LookAt response and indicator
          (`self.SetComponentResponseToInteractCollision`)
          (`self.SetupInteractionIndicator`))
        (:`NewEnumerator2`
          (setmembers `/Game/BP/Data/Structs/F_InteractionData` :`StructRef` (`self.InteractionData`) :`TriggerInteractionByTouch` false)
          ; Create a sphere collision component and set the sphere radius when the interaction type is set to overlap
          (bind _returnvalue (`|AddComponentByClass` (`self.GetOwner`) "/Script/Engine.SphereComponent" false (`KismetMathLibrary.MakeTransform` (0.0 0.0 0.0))))
          (`SphereComponent.SetSphereRadius` _returnvalue (`self.InteractionRadius`) true)
          ; Bind reaction to when the owning actor is overlapped by the player character
          (add `PrimitiveComponent.OnComponentBeginOverlap` _returnvalue (delegate `OnComponentBeginOverlap_Event`))
          ; Bind reaction to when the owning actor is overlapped by the player character
          (add `PrimitiveComponent.OnComponentEndOverlap` _returnvalue (delegate `OnComponentEndOverlap_Event`)))))
    (:`then_1`
      ; Set interaction highlight type for owning actor // Bind event if CanInteractByOverlap is true
      (`self.SetInteractionHighlightType`)
      (if (`.TriggerInteractionByTouch_31_196942BF4BFB01EE8AFE0CBC0E7066D1` (break `/Game/BP/Data/Structs/F_InteractionData` (`self.InteractionData`)))
        (add `Actor.OnActorBeginOverlap` (`self.GetOwner`) (`|CreateDelegate` :!event `OnActorBeginOverlap_Event`))))))

(event `OnComponentBeginOverlap_Event`
  (params (OverlappedComponent :type "PrimitiveComponent Object Reference") (OtherActor :type "Actor Object Reference") (OtherComp :type "PrimitiveComponent Object Reference") (OtherBodyIndex :type Integer) (bFromSweep :type Boolean) (SweepResult :type "HitResult Structure (by ref)"))
  ; Bind reaction to when the owning actor is overlapped by the player character
  (bind _instigator (`Actor.Instigator` OtherActor)
    (:`then`
      (if (`Pawn.IsPlayerControlled` _instigator)
        (bind _returnvalue (`PlayerState.GetPlayerController` (`Pawn.PlayerState` _instigator)))
        (`self.SetShowAsInteractable` true _returnvalue)
        (message `/Game/BP/Interfaces/BPI_Interaction.SetOverlapInteractionActor` _returnvalue (`self.GetOwner`) true)))
    (:`else`)))

(event `OnComponentEndOverlap_Event`
  (params (OverlappedComponent :type "PrimitiveComponent Object Reference") (OtherActor :type "Actor Object Reference") (OtherComp :type "PrimitiveComponent Object Reference") (OtherBodyIndex :type Integer))
  ; Bind reaction to when the owning actor is overlapped by the player character
  (bind _instigator (`Actor.Instigator` OtherActor)
    (:`then`
      (if (`Pawn.IsPlayerControlled` _instigator)
        (bind _returnvalue (`PlayerState.GetPlayerController` (`Pawn.PlayerState` _instigator)))
        (`self.SetShowAsInteractable` false _returnvalue)
        (message `/Game/BP/Interfaces/BPI_Interaction.SetOverlapInteractionActor` _returnvalue null false)))
    (:`else`)))

(event `OnActorBeginOverlap_Event`
  (params (OverlappedActor :type "Actor Object Reference") (OtherActor :type "Actor Object Reference"))
  ; Pickup interactable by touch // Can only be triggered by player pawn
  (bind _instigator (`Actor.Instigator` OtherActor)
    (:`then`
      (if (`Pawn.IsPlayerControlled` _instigator)
        (`self.OnInteractedWith` (`PlayerState.GetPlayerController` (`Pawn.PlayerState` _instigator)))))
    (:`else`)))

(event `SetShowAsInteractable`
  (params (ShowAsInteractable :type Boolean) (InteractingController :type "PlayerController Object Reference"))
  ; Show interaction text and highlights / outlines
  (if ShowAsInteractable
    (`/Engine/EditorBlueprintResources/StandardMacros.DoOnce` false :!label _label
      (:`Completed`
        (`self.CheckInteractionDisplayType`)
        (`self.HighlightInteractable` true)
        (message `/Game/BP/Interfaces/BPI_Interaction.UpdateHUD_Interaction` (`PlayerController.GetHUD` InteractingController) (`self.AddKeybindToInteractionText` InteractingController) (`self.GetOwner`))))
    (else
      (`|ExecutionSequence`
        (:`then_0`
          (`self.HighlightInteractable` false)
          (message `/Game/BP/Interfaces/BPI_Interaction.UpdateHUD_Interaction` (`PlayerController.GetHUD` InteractingController) (struct) null))
        (:`then_1`
          (goto _label :!via `Reset`))))))

(fn `AddKeybindToInteractionText`
  (params (InteractingController :type "PlayerController Object Reference"))
  (returns (InteractionData :type "/Game/BP/Data/Structs/F_InteractionData Structure"))
  (locals (Local_InteractionData :type "/Game/BP/Data/Structs/F_InteractionData Structure"))
  (bind _interactionkeybind (message `/Game/BP/Interfaces/BPI_Interaction.GetInteractionKeybind` InteractingController))
  (bind _output_get (set `local.Local_InteractionData` (`self.InteractionData`)))
  (bind _structout (setmembers `/Game/BP/Data/Structs/F_InteractionData` :`StructRef` _output_get :`InteractionText` (`|FormatText` "Press {key} to {info}" _interactionkeybind (`.InteractionText_10_FF976C594332CC1073637B91369ED674` (break `/Game/BP/Data/Structs/F_InteractionData` _output_get)))))
  (return _structout))

(fn `HighlightInteractable`
  (params (EnableCustomDepth :type Boolean))
  (for _array_element (`Actor.GetComponentsByTag` (`self.GetOwner`) "/Script/Engine.PrimitiveComponent" "Interact")
    (`PrimitiveComponent.SetRenderCustomDepth` _array_element (`local.EnableCustomDepth`))))

(fn `IsInteractableComponent`
  (params (Component :type "ActorComponent Object Reference"))
  (returns (ReturnValue :type Boolean))
  (return (`self.ComponentHasTag` Component "Interact")))

(fn `SetComponentResponseToInteractCollision`
  (for _array_element (`Actor.K2_GetComponentsByClass` (`self.GetOwner`) "/Script/Engine.PrimitiveComponent")
    (`PrimitiveComponent.SetCollisionResponseToChannel` _array_element "ECC_GameTraceChannel1" (select `bool` (`self.ComponentHasTag` _array_element "Interact") :`false` "ECR_Ignore" :`true` "ECR_Block" :!type "ECollisionResponse Enum"))))

(fn `SetInteractionHighlightType`
  (for _array_element (`Actor.GetComponentsByTag` (`self.GetOwner`) "/Script/Engine.PrimitiveComponent" "Interact")
    (`PrimitiveComponent.SetCustomDepthStencilValue` _array_element (`KismetMathLibrary.Conv_ByteToInt` (`.InteractionHighlightType_14_60C495F143D873594F97FCA5D716B377` (break `/Game/BP/Data/Structs/F_InteractionData` (`self.InteractionData`)))))))

(fn `SetupInteractionIndicator`
  (`self.EnableInteractionIndicator`
    (:`then`
      (bind _returnvalue (`|AddComponentByClass` (`self.GetOwner`) "/Script/Engine.MaterialBillboardComponent" false (`KismetMathLibrary.MakeTransform` (`self.InteractionIndicatorLocation`))))
      (`MaterialBillboardComponent.AddElement` _returnvalue "/Game/Materials/PARENTS/M_InteractionIndicator.M_InteractionIndicator" null false 3.0 3.0 null)
      (`PrimitiveComponent.SetDefaultCustomPrimitiveDataVector4` _returnvalue 0 (`/Game/BP/FunctionsAndMacros/BFL_Helpers.LinearColorToVector4` (`KismetMathLibrary.SelectColor` (`/Game/BP/FunctionsAndMacros/BFL_Helpers.GetColorFromRarity` (`.Rarity_30_F1070BF740E8FCD6F3638EB41805775A` (break `/Game/BP/Data/Structs/F_InteractionData` (`self.InteractionData`)))) (struct :`R` 1.0 :`G` 1.0 :`B` 1.0 :`A` 1.0) (`self.InteractionIndicatorColorByRarity`)))))
    (:`else`)))