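; Editor utility actor that renders item icons from data assets and saves them as UI textures.
; The construction script builds the item mesh, zeroes material bob and rotation, and configures the camera, scene capture and cutoff distance in a material parameter collection.
; CaptureIcon clears the render target and captures only that mesh.
; SaveIconToDisk converts the target to a static texture named after the item, in the UI texture group.
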(fn `CaptureIcon`
  (bind _scenecapturecomponent2d (`self.SceneCaptureComponent2D`))
  (`KismetRenderingLibrary.ClearRenderTarget2D` (`SceneCaptureComponent2D.TextureTarget` _scenecapturecomponent2d) (struct))
  (set `SceneCaptureComponent.bCaptureEveryFrame` true _scenecapturecomponent2d)
  (`SceneCaptureComponent.ShowOnlyComponent` _scenecapturecomponent2d (`self.StaticMesh`))
  (`SceneCaptureComponent2D.CaptureScene` _scenecapturecomponent2d)
  (set `SceneCaptureComponent.bCaptureEveryFrame` false _scenecapturecomponent2d))

(fn `SaveIconToDisk`
  (bind _itemdata (`self.ItemData`)
    (:`then`
      (bind _returnvalue (`KismetRenderingLibrary.RenderTargetCreateStaticTexture2DEditorOnly` (`SceneCaptureComponent2D.TextureTarget` (`self.SceneCaptureComponent2D`)) (`KismetStringLibrary.Concat_StrStr` "/Game/Materials/Textures/UI/T_UI_" (`KismetTextLibrary.Conv_TextToString` (`.Name_2_1346FB0E4E0D52F483ACEC934DB39AE6` (break `/Game/BP/Data/Structs/F_InteractionData` (`/Game/BP/Data/DataAssets/000_Primary/PDA_Item. InteractionData` _itemdata)))))))
      (set `Texture.LODGroup` "TEXTUREGROUP_UI" _returnvalue))
    (:`else`)))

(fn `SetupStaticMesh`
  (bind _staticmesh (`self.StaticMesh`))
  ; Setup static mesh from data asset
  (bind _itemdata (`self.ItemData`)
    (:`then`
      (`/Game/BP/Data/DataAssets/000_Primary/PDA_Item.SetUpStaticMesh` _itemdata _staticmesh)
      ;;[0 0 0 0.5] Remove rotation and bob, if applied
      (`MeshComponent.SetScalarParameterValueOnMaterials` _staticmesh "MF_Bob_BobAmount" 0.0)
      (`MeshComponent.SetScalarParameterValueOnMaterials` _staticmesh "MF_Rot_RotationTime" 0.0))
    (:`else`)))

(fn `UserConstructionScript`
  (`self.SetupStaticMesh`)
  ; Set relative transform of static mesh
  (`SceneComponent.K2_SetRelativeTransform` (`self.StaticMesh`) (`self.MeshTransform`) false false)
  ; Set capture source of the scene capture moment
  (set `SceneCaptureComponent.CaptureSource` (`self.CaptureSource`) (`self.SceneCaptureComponent2D`))
  ; Set the cull distance of the post process material
  (`KismetMaterialLibrary.SetScalarParameterValue` "/Game/Materials/MPC/MPC_IconCapture.MPC_IconCapture" "CutOffDistance" (`self.CutoffDistance`))
  ; Set FOV for camera and scene capture component
  (bind _output_get (set `SceneCaptureComponent2D.FOVAngle` (`self.FieldOfView`) (`self.SceneCaptureComponent2D`)))
  (set `CameraComponent.FieldOfView` _output_get (`self.Camera`)))